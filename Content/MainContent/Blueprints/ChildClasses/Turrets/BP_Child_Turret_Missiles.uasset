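; Missile turret child Blueprint that fires a staggered volley from its muzzle array, adding a fourth muzzle on BeginPlay.
; Firing blocks the player ship's switching, launches the first missile immediately, then loops a timer to step through the remaining muzzles.
; Each shot spawns through the owning ship's multicast projectile event.
; The last shot restores switching, clears the ship's projectile transforms and timer, and schedules the cooldown reset.
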(event `self.ReceiveBeginPlay`
  (`parent.ReceiveBeginPlay`)
  (`KismetArrayLibrary.Array_Add` (`self.Muzzle Array`) (`self.Muzzle Arrow 4`)))

(event `self.Event Fire Turret`
  (params (`Transform Array` :type "Array of Transform Structure (by ref)") (`Player Parent Ref` :type "/Game/MainContent/Blueprints/ParentClasses/BP_Ship_Parent Object Reference"))
  (`parent.Event Fire Turret` `Transform Array` `Player Parent Ref`)
  (set `/Game/MainContent/Blueprints/ParentClasses/BP_Ship_Parent.Can Switch?` false `Player Parent Ref`)
  (`self.StaggerMissileFire`) ; Initial Shot
  (bind _returnvalue (`KismetSystemLibrary.K2_SetTimer` null "StaggerMissileFire" (`self.Shots Delay`) true))
  (set `self.Stagger Missiles TH` _returnvalue))

(fn `StaggerMissileFire`
  (bind _bp_ship_parent_ref (`self.BP Ship Parent Ref`))
  (bind _bp_ship_parent_ref_2 (`self.BP Ship Parent Ref`))
  (`/Game/MainContent/Blueprints/ParentClasses/BP_Ship_Parent.Event Spawn Projectile (Multicast)` _bp_ship_parent_ref (`SceneComponent.K2_GetComponentToWorld` (`|GetArrayItem` (`self.Muzzle Array`) (`self.Shots Int`))) self _bp_ship_parent_ref)
  (bind _result (`/Engine/EditorBlueprintResources/StandardMacros.IncrementInt` (`self.Shots Int`))
    (:`  `
      (if (>= _result (`KismetArrayLibrary.Array_Length` (`self.Muzzle Array`)))
        (set `self.Shots Int` 0)
        (set `/Game/MainContent/Blueprints/ParentClasses/BP_Ship_Parent.Can Switch?` true _bp_ship_parent_ref_2)
        (`KismetArrayLibrary.Array_Clear` (`/Game/MainContent/Blueprints/ParentClasses/BP_Ship_Parent.Projectile Transform Array` _bp_ship_parent_ref_2))
        (`KismetSystemLibrary.K2_ClearAndInvalidateTimerHandle` (`self.Stagger Missiles TH`))
        (`KismetSystemLibrary.K2_SetTimer` null "ClearCooldown" (`self.Cooldown Time`))
        (else
          (set `self.Shots Delay` 0.3))))))

(fn `UserConstructionScript`
  (`parent.UserConstructionScript`))