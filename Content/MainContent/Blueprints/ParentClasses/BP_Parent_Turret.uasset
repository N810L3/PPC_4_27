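; Parent Blueprint for ship turrets, providing selection, cursor aiming and firing logic.
; Selecting a turret runs on the owning client, shows its outline and passes its projectile class to the player's ship.
; Aiming intersects the mouse ray with a horizontal plane at turret height and returns a smoothly interpolated rotation.
; FireTurret only flags firing and stores the ship, while StandardFireTurret has that ship multicast-spawn projectiles per supplied transform.
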(event `Event Select Turret (Owning Client)`
  (`SceneComponent.SetVisibility` (`self.PS Turret Outline`) true false)
  (`KismetSystemLibrary.Delay` (`GameplayStatics.GetWorldDeltaSeconds`))
  (`self.SetProjectileClassBPI`))

(event `Event Deselect Turret (Owning Client)`
  (`SceneComponent.SetVisibility` (`self.PS Turret Outline`) false false))

(event `Event Fire Turret`
  (params (`Transform Array` :type "Array of Transform Structure") (`Player Parent Ref` :type "/Game/MainContent/Blueprints/ParentClasses/BP_Ship_Parent Object Reference"))
  (set `self.Is Firing?` true)
  (set `self.BP Ship Parent Ref` `Player Parent Ref`))

(fn `RotateTurret`
  (params (`Child BP` :type "SceneComponent Object Reference") (`Delta Time` :type "Float (double-precision)"))
  (returns (`New Rotation` :type "Rotator Structure"))
  (bind (_returnvalue_roll _returnvalue_pitch) (`KismetMathLibrary.BreakRotator` (`SceneComponent.K2_GetComponentRotation` `Child BP`)))
  (bind (_worldlocation _worlddirection) (`PlayerController.DeprojectMousePositionToWorld` (`GameplayStatics.GetPlayerController` 0)))
  (bind (_returnvalue_roll_2 _returnvalue_pitch_2 _returnvalue_yaw) (`KismetMathLibrary.BreakRotator` (`KismetMathLibrary.FindLookAtRotation` (`SceneComponent.K2_GetComponentLocation` `Child BP`) (`.Intersection` (`KismetMathLibrary.LinePlaneIntersection_OriginNormal` _worldlocation (+ _worldlocation (* _worlddirection 1000000.0)) (`self.K2_GetActorLocation`) (0.0 0.0 1.0))))))
  (return (`KismetMathLibrary.RInterpTo` (`self.K2_GetActorRotation`) (`KismetMathLibrary.MakeRotator` _returnvalue_roll _returnvalue_pitch _returnvalue_yaw) (`local.Delta Time`) (`self.Turret Rotate Speed`))))

(fn `SetProjectileClass`
  (params (`Projectile Class` :type "/Game/MainContent/Blueprints/ParentClasses/BP_Projectile_Parent Class Reference")))

(fn `SetProjectileClassBPI`
  (message `/Game/MainContent/Blueprints/BPInterfaces/BPI_SetProjectileClass.SetProjectileClass` (cast `/Game/MainContent/Blueprints/ParentClasses/BP_Ship_Parent` (`GameplayStatics.GetPlayerPawn` 0) :!pure true) (`self.Turret's Projectile Class`)))

(fn `StandardFireTurret`
  (params (`Transform Array` :type "Array of Transform Structure"))
  (bind _bp_ship_parent_ref (`self.BP Ship Parent Ref`))
  (for _array_element `Transform Array`
    (`/Game/MainContent/Blueprints/ParentClasses/BP_Ship_Parent.Event Spawn Projectile (Multicast)` _bp_ship_parent_ref _array_element self _bp_ship_parent_ref))
  (bind _bp_ship_parent_ref_2 (`self.BP Ship Parent Ref`)
    (:`then`
      (`KismetArrayLibrary.Array_Clear` (`/Game/MainContent/Blueprints/ParentClasses/BP_Ship_Parent.Projectile Transform Array` _bp_ship_parent_ref_2)))
    (:`else`)))

(fn `UserConstructionScript`
  (set `self.Muzzle Array` (`|MakeArray` (`self.Muzzle Arrow 1`) (`self.Muzzle Arrow 2`) (`self.Muzzle Arrow 3`))))