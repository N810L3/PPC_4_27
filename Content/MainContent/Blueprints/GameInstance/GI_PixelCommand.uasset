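; Game instance for Pixel Command that hosts, finds and joins multiplayer sessions, with separate LAN flags for hosting and finding.
; Hosting ignores its connection-count input for a fixed maximum, then issues a console open command for Level_Blank as a listen server.
; Finding appends results to SessionsArray and notifies the main menu's join widget, reached through the HUD.
; Joining stores the chosen session, prints its details and hides the loading bar on failure.
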(event `Event Host Session`
  (params (PublicConnections :type Integer))
  (`CreateSessionCallbackProxy.CreateSession` (`GameplayStatics.GetPlayerController` 0) 999999 (`self.Use LAN Host?`)
    (:`then`
      (`KismetSystemLibrary.PrintString` (`KismetStringLibrary.Concat_StrStr` "Using LAN? " (`KismetStringLibrary.Conv_BoolToString` (`self.Use LAN Host?`))) true true (struct :`R` 1.0 :`G` 0.010379 :`A` 1.0)))
    (:`OnSuccess`
      (`KismetSystemLibrary.PrintString` "Session Success! \n:D" true true (struct :`R` 0.001298 :`G` 1.0 :`A` 1.0))
      (`KismetSystemLibrary.ExecuteConsoleCommand` (`KismetStringLibrary.Concat_StrStr` "open " "Level_Blank" "?listen") (`GameplayStatics.GetPlayerController` 0)))
    (:`OnFailure`
      (`KismetSystemLibrary.PrintString` "Session Failed!!! \n>:c" true true (struct :`R` 1.0 :`G` 0.010379 :`A` 1.0)))))

(event `Event Find Session`
  (bind _results (`FindSessionsCallbackProxy.FindSessions` (`GameplayStatics.GetPlayerController` 0) 999999 (`self.Use LAN Find?`))
    (:`then`
      (`KismetSystemLibrary.PrintString` (`KismetStringLibrary.Concat_StrStr` "Using LAN? " (`KismetStringLibrary.Conv_BoolToString` (`self.Use LAN Find?`))) true true (struct :`R` 1.0 :`G` 0.010379 :`A` 1.0))
      (`KismetSystemLibrary.PrintString` "Finding Sessions..."))
    (:`OnSuccess`
      (`KismetSystemLibrary.PrintString` "Session Found! \n:D" true true (struct :`R` 0.001298 :`G` 1.0 :`A` 1.0))
      (for _array_element _results
        (bind _output_get (set `self.Blueprint Session` _array_element))
        (`KismetArrayLibrary.Array_Add` (`self.Sessions Array`) _output_get))
      (`self.HideLoadingBar` :!label _label)
      (`/Game/MainContent/Widgets/MainMenu/W_Menu_Find.Event Found Sessions` (`/Game/MainContent/Widgets/MainMenu/W_Menu_Main.W_Menu_Join` (`self.GetMainMenuRef`))))
    (:`OnFailure`
      (`KismetSystemLibrary.PrintString` "Session Failed!!! \n>:c" true true (struct :`R` 1.0 :`G` 0.010379 :`A` 1.0))
      (goto _label))))

(event `Event Join Session`
  (params (SearchResult :type "BlueprintSessionResult Structure (by ref)"))
  (bind _session_joining (`self.Session Joining`))
  (bind _output_get (set `self.Session Joining` SearchResult))
  (`JoinSessionCallbackProxy.JoinSession` (`GameplayStatics.GetPlayerController` 0) _output_get
    (:`OnSuccess`
      (`KismetSystemLibrary.PrintString` "Session Join! \n:D" true true (struct :`R` 0.001298 :`G` 1.0 :`A` 1.0)))
    (:`OnFailure`
      (`KismetSystemLibrary.PrintString` "Session Failed!!! \n>:c" true true (struct :`R` 1.0 :`G` 0.010379 :`A` 1.0))
      (`self.HideLoadingBar`)))
  (`KismetSystemLibrary.PrintString` (`KismetTextLibrary.Conv_TextToString` (`|FormatText` "Server Name: {SN} \nMax Players: {MP} \nCurrent Players: {CP} \nPing: {PG}" (`FindSessionsCallbackProxy.GetServerName` _session_joining) (`FindSessionsCallbackProxy.GetMaxPlayers` _session_joining) (`FindSessionsCallbackProxy.GetCurrentPlayers` _session_joining) (`FindSessionsCallbackProxy.GetPingInMs` _session_joining))) true true (struct :`R` 1.0 :`B` 0.941021 :`A` 1.0) 10.0))

(fn `GetMainMenuRef`
  (returns (`Main Menu Ref` :type "/Game/MainContent/Widgets/MainMenu/W_Menu_Main Object Reference"))
  (return (`/Game/MainContent/Blueprints/HUDs/HUD_MainMenu.Main Menu Ref` (cast `/Game/MainContent/Blueprints/HUDs/HUD_MainMenu` (`PlayerController.GetHUD` (`GameplayStatics.GetPlayerController` 0)) :!pure true))))

(fn `HideLoadingBar`
  (`Widget.SetVisibility` (`/Game/MainContent/Widgets/MainMenu/W_Menu_Find.HorizontalBox_Loading` (`/Game/MainContent/Widgets/MainMenu/W_Menu_Main.W_Menu_Join` (`self.GetMainMenuRef`))) "Hidden"))