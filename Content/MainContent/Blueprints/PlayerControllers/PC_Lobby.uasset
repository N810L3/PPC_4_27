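; Player controller for the lobby that shows the mouse cursor and relays player list updates to the lobby UI.
; BeginPlay caches the lobby HUD and has a local-controller check with nothing attached.
; An owning-client event waits briefly, then forwards the player info to the HUD's lobby reference if the cached HUD is valid.
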(event `self.ReceiveBeginPlay`
  (bind _ashud_lobby (cast `/Game/MainContent/Blueprints/HUDs/HUD_Lobby` (`self.GetHUD`)))
  (set `self.HUD Lobby Ref` _ashud_lobby)
  (set `self.bShowMouseCursor` true)
  (if (`self.IsLocalPlayerController`)
    _))

(event `Event Update Player List (Owning Client)`
  (params (`Player Info Struct` :type "Array of /Game/MainContent/Blueprints/Structs/Struct_PlayerInfo Structure"))
  (`KismetSystemLibrary.Delay` 0.2)
  (bind _hud_lobby_ref (`self.HUD Lobby Ref`)
    (:`then`
      (`/Game/MainContent/Widgets/Lobby/W_Lobby_Main.Event Update Player List` (`/Game/MainContent/Blueprints/HUDs/HUD_Lobby.Lobby Ref` _hud_lobby_ref) `Player Info Struct`))
    (:`else`)))

(fn `UserConstructionScript`)