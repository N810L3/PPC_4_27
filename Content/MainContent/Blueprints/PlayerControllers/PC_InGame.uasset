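; In-game player controller that requests a spawn for its player in the TDM game mode.
; On BeginPlay it shows the mouse cursor and sets game-only input, then the local controller calls a server RPC.
; The server event casts the game mode to GM_TDM and has it spawn the player at a random location.
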(event `self.ReceiveBeginPlay`
  (set `self.bShowMouseCursor` true)
  (`WidgetBlueprintLibrary.SetInputMode_GameOnly` self)
  (if (`self.IsLocalPlayerController`)
    (`self.Event Spawn Player (On Server)`)))

(event `Event Spawn Player (On Server)`
  (bind _asgm_tdm (cast `/Game/MainContent/Blueprints/Gamemodes/GM_TDM` (`GameplayStatics.GetGameMode`)))
  (`/Game/MainContent/Blueprints/Gamemodes/GM_TDM.SpawnPlayerRandomLocation` _asgm_tdm self))

(fn `UserConstructionScript`)