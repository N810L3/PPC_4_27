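; GM_TDM is a game mode that tracks joining player controllers and provides random ship spawning, with no team or scoring logic.
; PostLogin only stores each controller; SpawnPlayerRandomLocation, not called here, destroys the current pawn, then spawns and possesses a BP_Ship_Parent.
; GetRandomPlayerStart offsets a random PlayerStart horizontally within a box.
; Its location, rotation and scale roll separate random indices, so can come from different starts.
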(event `self.K2_PostLogin`
  (params (NewPlayer :type "PlayerController Object Reference"))
  (`KismetArrayLibrary.Array_Add` (`self.Player Controllers Array`) NewPlayer))

(fn `GetRandomPlayerStart`
  (returns (`Spawn Transform` :type "Transform Structure"))
  (bind _outactors (`GameplayStatics.GetAllActorsOfClass` "/Script/Engine.PlayerStart"))
  (bind _output_get (set `self.Player Start Array` _outactors))
  (bind (_returnvalue_location _returnvalue_rotation _returnvalue_scale) (`KismetMathLibrary.BreakTransform` (`self.GetTransform` (`|GetArrayItem` (`self.Player Start Array`) (`KismetMathLibrary.RandomIntegerInRange` 0 (- (`KismetArrayLibrary.Array_Length` _output_get) 1))))))
  (return (`KismetMathLibrary.MakeTransform` (`KismetMathLibrary.RandomPointInBoundingBox` _returnvalue_location (500.0 500.0 0.0)) _returnvalue_rotation _returnvalue_scale)))

(fn `SpawnPlayerRandomLocation`
  (params (`Player Controler` :type "PlayerController Object Reference"))
  (bind _returnvalue (`Controller.K2_GetPawn` `Player Controler`))
  (`/Engine/EditorBlueprintResources/StandardMacros.IsValid` _returnvalue
    (:`Is Valid`
      (`self.K2_DestroyActor` _returnvalue))
    (:`Is Not Valid`
      _))
  (bind _returnvalue_2 (`|SpawnActorFromClass` "/Game/MainContent/Blueprints/ParentClasses/BP_Ship_Parent.BP_Ship_Parent_C" (`self.GetRandomPlayerStart`) "AlwaysSpawn" "OverrideRootScale" null null))
  (`/Engine/EditorBlueprintResources/StandardMacros.IsValid` _returnvalue_2
    (:`Is Valid`
      (`Controller.Possess` `Player Controler` _returnvalue_2)
      (`KismetSystemLibrary.PrintString` "Spawned!"))))

(fn `UserConstructionScript`)