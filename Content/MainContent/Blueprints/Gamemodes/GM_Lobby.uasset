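; GM_Lobby is the lobby game mode that tracks players as they connect.
; On PostLogin it casts the new controller to PC_Lobby, builds a player info struct from the PlayerState name, and stores both in arrays.
; It then loops over every stored controller and passes the full info list to its owning-client update event, refreshing each player list.
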(event `self.K2_PostLogin`
  (params (NewPlayer :type "PlayerController Object Reference"))
  (bind _aspc_lobby (cast `/Game/MainContent/Blueprints/PlayerControllers/PC_Lobby` NewPlayer))
  (`KismetArrayLibrary.Array_Add` (`self.Player Controllers Array`) _aspc_lobby)
  (bind _output_get (set `/Game/MainContent/Blueprints/PlayerControllers/PC_Lobby.Player Info Struct` (make `/Game/MainContent/Blueprints/Structs/Struct_PlayerInfo` :`Player Name` (`PlayerState.GetPlayerName` (`Controller.PlayerState` NewPlayer))) _aspc_lobby))
  (`KismetArrayLibrary.Array_Add` (`self.Connected Player Info Struct`) _output_get)
  (for _array_element (`self.Player Controllers Array`)
    (`/Game/MainContent/Blueprints/PlayerControllers/PC_Lobby.Event Update Player List (Owning Client)` _array_element (`self.Connected Player Info Struct`))))

(fn `UserConstructionScript`)